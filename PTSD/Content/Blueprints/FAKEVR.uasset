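; Player pawn that simulates VR with keyboard and mouse: WASD camera-relative walking, mouse look, and a rotatable, movable hand.
; Tick applies held-key movement flags, while key 2 line-traces from Holder to teleport onto Telepoint actors.
; Key 1 interacts with actors overlapping Holder: it grabs Balls, triggers KeyboardInputs, or ends DecisionUI choices.
; Decisions accumulate with start and end times in SaveText, seeded with name and date, and are printed on screen.
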(event EventTick
  (params (DeltaSeconds :type Float%20%28single-precision%29))
  (bind _capsule (Variables|Default|GetCapsule))
  (bind _cube (Variables|Default|GetCube))
  (bind _camera (Variables|Default|GetCamera))
  (bind _camera_2 (Variables|Default|GetCamera))
  (bind _camera_3 (Variables|Default|GetCamera))
  (bind _returnvalue (Transformation|GetWorldRotation _camera_3))
  (bind _returnvalue_2 (Math|Vector|GetRightVector _camera_2))
  (bind _returnvalue_3 (Math|Vector|GetForwardVector _camera))
  (bind _returnvalue_4 (* _returnvalue_2 5))
  (bind _returnvalue_5 (* _returnvalue_2 -5))
  (bind _returnvalue_6 (* _returnvalue_3 -5))
  (bind _returnvalue_7 (* _returnvalue_3 5))
  (Utilities|FlowControl|Sequence
    (:then_0
      ;[1 1 1] Body
      (Utilities|FlowControl|Sequence
        (:then_0
          (if (Variables|Default|GetWalkForward)
            (Transformation|AddLocalOffset _capsule (Math|Vector|MakeVector (.x _returnvalue_7) (.y _returnvalue_7) 0.0) false false)))
        (:then_1
          (if (Variables|Default|GetWalkBackward)
            (Transformation|AddLocalOffset _capsule (Math|Vector|MakeVector (.x _returnvalue_6) (.y _returnvalue_6) 0.0) false false)))
        (:then_2
          (if (Variables|Default|GetWalkLeft)
            (Transformation|AddLocalOffset _capsule (Math|Vector|MakeVector (.x _returnvalue_5) (.y _returnvalue_5) 0.0) false false)))
        (:then_3
          (if (Variables|Default|GetWalkRight)
            (Transformation|AddLocalOffset _capsule (Math|Vector|MakeVector (.x _returnvalue_4) (.y _returnvalue_4) 0.0) false false)))))
    (:then_1
      ;[1 1 1] Hand Movement
      (Utilities|FlowControl|Sequence
        (:then_0
          (if (Variables|Default|GetUseHand)
            (if (Variables|Default|GetRotate%20Left)
              (Transformation|AddLocalRotation _cube "0, 0,-10.000000" false false))))
        (:then_1
          (if (Variables|Default|GetUseHand)
            (if (Variables|Default|GetRotate%20Right)
              (Transformation|AddLocalRotation _cube "0, 0,10.000000" false false))))
        (:then_2
          (if (Variables|Default|GetUseHand)
            (Transformation|AddLocalOffset _cube (Math|Vector|MakeVector (Class|Actor|GetInputAxisKeyValue) (Class|Actor|GetInputAxisKeyValue) 0.0) false false)))
        (:then_3
          (Transformation|AddLocalRotation _camera_3 (Math|Rotator|MakeRotator 0.0 (Class|Actor|GetInputAxisKeyValue) (Class|Actor|GetInputAxisKeyValue)) false false)
          (Transformation|SetWorldRotation _camera_3 (Math|Rotator|MakeRotator 0.0 (.pitch _returnvalue) (.yaw _returnvalue)) false false))))
    (:then_2
      (if (Variables|Default|GetInteracting)
        (Variables|Default|SetHolder%20Transform (Transformation|GetWorldTransform (Variables|Default|GetBox)))))))

(event EventBeginPlay
  (Variables|Default|SetSaveText (Utilities|String|Append (Variables|Default|GetSaveText) (Variables|Default|GetName) " 
" "Date: " (Variables|Default|GetDate) " 
" "Decisions ----------------------------------" " 
")))

(event Input|MouseEvents|MouseWheelAxis
  (params (AxisValue :type Float%20%28single-precision%29))
  ;[1 1 1] Hand Movement
  (Transformation|AddLocalRotation (Variables|Default|GetCube) (Math|Rotator|MakeRotator 0.0 (* -10 AxisValue) 0.0) false false))

(event Input|KeyboardEvents|2
  (params (Key :type Key%20Structure :default "AnyKey"))
  (bind _holder (Variables|Default|GetHolder))
  (bind _returnvalue (Transformation|GetWorldLocation _holder))
  ;[1 1 1] Teleport
  (:Pressed
    (bind _outhit (Collision|LineTraceByChannel _returnvalue (+ _returnvalue (* (Math|Vector|GetForwardVector (Transformation|GetWorldRotation _holder)) 10000)) "TraceTypeQuery1" false 0 "Persistent"))
    (if (== (Utilities|GetClass (.HitActor (Collision|BreakHitResult _outhit))) "/Game/Blueprints/Telepoint.Telepoint_C")
      (Transformation|Teleport (Math|Vector|MakeVector (.x (.Location (Math|Transform|BreakTransform (Transformation|GetActorTransform (.HitActor (Collision|BreakHitResult _outhit)))))) (.y (.Location (Math|Transform|BreakTransform (Transformation|GetActorTransform (.HitActor (Collision|BreakHitResult _outhit)))))) (.z (.location (Transformation|GetActorTransform)))) (.Rotation (Math|Transform|BreakTransform (Transformation|GetActorTransform (.HitActor (Collision|BreakHitResult _outhit)))))))))

(event Input|KeyboardEvents|5
  (params (Key :type Key%20Structure :default "AnyKey"))
  (:Pressed
    (Variables|Default|SetUseHand true))
  (:Released
    (Variables|Default|SetUseHand false)))

(event Input|KeyboardEvents|A
  (params (Key :type Key%20Structure :default "AnyKey"))
  (:Pressed
    (Variables|Default|SetWalkLeft true))
  (:Released
    (Variables|Default|SetWalkLeft false)))

(event Input|KeyboardEvents|S
  (params (Key :type Key%20Structure :default "AnyKey"))
  (:Pressed
    (Variables|Default|SetWalkBackward true))
  (:Released
    (Variables|Default|SetWalkBackward false)))

(event Input|KeyboardEvents|D
  (params (Key :type Key%20Structure :default "AnyKey"))
  (:Pressed
    (Variables|Default|SetWalkRight true))
  (:Released
    (Variables|Default|SetWalkRight false)))

(event Input|KeyboardEvents|W
  (params (Key :type Key%20Structure :default "AnyKey"))
  (:Pressed
    (Variables|Default|SetWalkForward true))
  (:Released
    (Variables|Default|SetWalkForward false)))

(event Input|KeyboardEvents|4
  (params (Key :type Key%20Structure :default "AnyKey"))
  (:Pressed
    (Variables|Default|SetRotate%20Left true))
  (:Released
    (Variables|Default|SetRotate%20Left false)))

(event Input|KeyboardEvents|6
  (params (Key :type Key%20Structure :default "AnyKey"))
  (:Pressed
    (Variables|Default|SetRotate%20Right true))
  (:Released
    (Variables|Default|SetRotate%20Right false)))

(event Input|KeyboardEvents|1
  (params (Key :type Key%20Structure :default "AnyKey"))
  (:Pressed
    (Variables|Default|SetInteracting true)
    (for _array_element (Collision|GetOverlappingActors (Variables|Default|GetHolder) 0 :!class /Script/Engine.PrimitiveComponent)
      (if (Variables|Default|GetInteracting)
        (bind _output_get (Variables|Default|SetInteracted%20Object _array_element))
        (if (== (Utilities|GetClass _array_element) "/Game/Blueprints/Ball.Ball_C")
          (bind _asball (Utilities|Casting|CastToBall _output_get))
          (Variables|/Game/Blueprints/Ball.Ball_C|SetHolder _asball self)
          (Variables|/Game/Blueprints/Ball.Ball_C|SetInteracted _asball true)
          (elif (== (Utilities|GetClass _array_element) "/Game/Blueprints/DecisionUI.DecisionUI_C")
            (bind _asdecision_ui (Utilities|Casting|CastToDecisionUI _output_get))
            (Variables|Default|SetSaveText (Utilities|String|Append (Variables|Default|GetSaveText) (Variables|/Game/Blueprints/DecisionUI.DecisionUI_C|GetDecisionName _asdecision_ui) " "))
            (Utilities|FlowControl|Sequence
              (:then_0
                (if (Variables|/Game/Blueprints/DecisionUI.DecisionUI_C|GetDecision1Bool _asdecision_ui)
                  (Variables|Default|SetSaveText (Utilities|String|Append (Variables|Default|GetSaveText) (Utilities|String|ToString(Text) (Variables|/Script/Engine.TextRenderComponent|GetText (Variables|/Game/Blueprints/DecisionUI.DecisionUI_C|GetDecisionText1 _asdecision_ui)))))
                  (bind _output_get_2 (Variables|Default|SetSaveText (Utilities|String|Append (Variables|Default|GetSaveText) " StartTime: " (Variables|/Game/Blueprints/DecisionUI.DecisionUI_C|GetStartTime _asdecision_ui) " EndTime: " (Utilities|String|ToString(Float) (Utilities|Time|GetTimeSeconds)) "  
") :!label _label))
                  (Development|PrintString _output_get_2 true true "(R=0.000000,G=0.660000,B=1.000000,A=1.000000)" 15.0)
                  (Default|EndDecision _asdecision_ui)
                  (Variables|Default|SetInteracting false)
                  (Default|EndObject _asball)))
              (:then_1
                (if (Variables|/Game/Blueprints/DecisionUI.DecisionUI_C|GetDecision2Bool _asdecision_ui)
                  (Variables|Default|SetSaveText (Utilities|String|Append (Variables|Default|GetSaveText) (Utilities|String|ToString(Text) (Variables|/Script/Engine.TextRenderComponent|GetText (Variables|/Game/Blueprints/DecisionUI.DecisionUI_C|GetDecisionText2 _asdecision_ui)))))
                  (goto _label)))
              (:then_2
                (if (Variables|/Game/Blueprints/DecisionUI.DecisionUI_C|GetDecision3Bool _asdecision_ui)
                  (Variables|Default|SetSaveText (Utilities|String|Append (Variables|Default|GetSaveText) (Utilities|String|ToString(Text) (Variables|/Script/Engine.TextRenderComponent|GetText (Variables|/Game/Blueprints/DecisionUI.DecisionUI_C|GetDecisionText3 _asdecision_ui)))))
                  (goto _label)))
              (:then_3
                (if (Variables|/Game/Blueprints/DecisionUI.DecisionUI_C|GetDecision4Bool _asdecision_ui)
                  (Variables|Default|SetSaveText (Utilities|String|Append (Variables|Default|GetSaveText) (Utilities|String|ToString(Text) (Variables|/Script/Engine.TextRenderComponent|GetText (Variables|/Game/Blueprints/DecisionUI.DecisionUI_C|GetDecisionText4 _asdecision_ui)))))
                  (goto _label))))
            (elif (== (Utilities|GetClass _array_element) "/Game/Blueprints/KeyboardInput.KeyboardInput_C")
              (bind _askeyboard_input (Utilities|Casting|CastToKeyboardInput _output_get))
              (Default|Interact _askeyboard_input))))))))

(fn ConstructionScript)