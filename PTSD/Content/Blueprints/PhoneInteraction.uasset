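; VR phone actor that plays a short branching telemarketer call addressed to the player by name.
; A Step counter advances on interact while an overlap flag is set, with two answer boxes setting the accept-or-decline Decision.
; Declining early ends the call, while reaching the final step calls CheckDecisions on the VRPawn before destroying the actor.
; Tick cycles four phone icon sprites through a Delay until the phone is answered.
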(event OnComponentBeginOverlap(Box)
  (params (OverlappedComponent :type Primitive%20Component%20Object%20Reference) (OtherActor :type Actor%20Object%20Reference) (OtherComp :type Primitive%20Component%20Object%20Reference) (OtherBodyIndex :type Integer) (bFromSweep :type Boolean) (SweepResult :type Hit%20Result%20Structure%20%28by%20ref%29))
  (Variables|Default|SetOn true))

(event OnComponentEndOverlap(Box)
  (params (OverlappedComponent :type Primitive%20Component%20Object%20Reference) (OtherActor :type Actor%20Object%20Reference) (OtherComp :type Primitive%20Component%20Object%20Reference) (OtherBodyIndex :type Integer))
  (Variables|Default|SetOn false))

(event OnComponentBeginOverlap(Box1)
  (params (OverlappedComponent :type Primitive%20Component%20Object%20Reference) (OtherActor :type Actor%20Object%20Reference) (OtherComp :type Primitive%20Component%20Object%20Reference) (OtherBodyIndex :type Integer) (bFromSweep :type Boolean) (SweepResult :type Hit%20Result%20Structure%20%28by%20ref%29))
  (Variables|Default|SetOn true)
  (Variables|Default|SetDecision true))

(event OnComponentEndOverlap(Box1)
  (params (OverlappedComponent :type Primitive%20Component%20Object%20Reference) (OtherActor :type Actor%20Object%20Reference) (OtherComp :type Primitive%20Component%20Object%20Reference) (OtherBodyIndex :type Integer))
  (Variables|Default|SetOn false))

(event OnComponentBeginOverlap(Box2)
  (params (OverlappedComponent :type Primitive%20Component%20Object%20Reference) (OtherActor :type Actor%20Object%20Reference) (OtherComp :type Primitive%20Component%20Object%20Reference) (OtherBodyIndex :type Integer) (bFromSweep :type Boolean) (SweepResult :type Hit%20Result%20Structure%20%28by%20ref%29))
  (Variables|Default|SetOn true)
  (Variables|Default|SetDecision false))

(event OnComponentEndOverlap(Box2)
  (params (OverlappedComponent :type Primitive%20Component%20Object%20Reference) (OtherActor :type Actor%20Object%20Reference) (OtherComp :type Primitive%20Component%20Object%20Reference) (OtherBodyIndex :type Integer))
  (Variables|Default|SetOn false))

(event Custom|interact
  (bind _decision (Variables|Default|GetDecision))
  (if (Variables|Default|GetOn)
    (switch int (Variables|Default|Getstep)
      (:0
        (Components|DestroyComponent (Variables|Default|GetBox))
        (Variables|Default|Setstep 1)
        (Collision|SetCollisionEnabled (Variables|Default|GetBox2) "QueryOnly")
        (Rendering|SetVisibility (Variables|Default|GetPlane) true true))
      (:1
        (if _decision
          (Rendering|SetVisibility (Variables|Default|GetText%20box) true true)
          (bind _asvrpawn (Utilities|Casting|CastToVRPawn (Game|Player|GetPlayerPawn 0))
            (:then
              (bind _output_get (Variables|Default|SetPhoneText (Utilities|String|Append "Hello, is this " (Variables|/Game/Blueprints/VRPawn.VRPawn_C|GetName _asvrpawn) "?")))
              (Rendering|Components|TextRender|SetText (Variables|Default|GetTextRender) (Utilities|Text|ToText(String) _output_get)))
            (:CastFailed
              _))
          (Components|DestroyComponent (Variables|Default|GetPlane))
          (Variables|Default|Setstep 2)
          (else
            (Actor|DestroyActor))))
      (:2
        (if _decision
          (Rendering|Components|TextRender|SetText (Variables|Default|GetTextRender) (Utilities|Text|ToText(String) "How would you like a time share in Sunny Orlando Florida!"))
          (Rendering|Components|TextRender|SetText (Variables|Default|GetTextRender1) (Utilities|Text|ToText(String) "No thank you"))
          (Rendering|Components|TextRender|SetText (Variables|Default|GetTextRender2) (Utilities|Text|ToText(String) "Hang Up"))
          (Variables|Default|Setstep 3)
          (else
            (Rendering|Components|TextRender|SetText (Variables|Default|GetTextRender) (Utilities|Text|ToText(String) "Sorry to bother you, good bye."))
            (Utilities|FlowControl|Delay 3.0)
            (Actor|DestroyActor))))
      (:3
        (bind _asvrpawn_2 (Utilities|Casting|CastToVRPawn (Game|Player|GetPlayerPawn 0)))
        (Default|CheckDecisions _asvrpawn_2)
        (Actor|DestroyActor)))))

(event EventBeginPlay
  (Rendering|SetVisibility (Variables|Default|GetText%20box) false true)
  (Collision|SetCollisionEnabled (Variables|Default|GetBox1) "NoCollision"))

(event Collision|EventActorBeginOverlap
  (params (OtherActor :type Actor%20Object%20Reference)))

(event EventTick
  (params (DeltaSeconds :type Float%20%28single-precision%29))
  (bind _phonesprite (Variables|Default|GetPhoneSprite))
  (Utilities|FlowControl|Sequence
    (:then_0
      (if (< (Variables|Default|Getstep) 1)
        (Utilities|FlowControl|Delay 0.8)
        (switch int (Variables|Default|GetFrame)
          (:0
            (Rendering|Components|Sprite|SetSprite _phonesprite "/Game/Textures/UI/Cell_Phone_Icon_Sprite_0.Cell_Phone_Icon_Sprite_0")
            (Variables|Default|SetFrame 1))
          (:1
            (Rendering|Components|Sprite|SetSprite _phonesprite "/Game/Textures/UI/Cell_Phone_Icon_Sprite_1.Cell_Phone_Icon_Sprite_1")
            (Variables|Default|SetFrame 2))
          (:2
            (Rendering|Components|Sprite|SetSprite _phonesprite "/Game/Textures/UI/Cell_Phone_Icon_Sprite_2.Cell_Phone_Icon_Sprite_2")
            (Variables|Default|SetFrame 3))
          (:3
            (Rendering|Components|Sprite|SetSprite _phonesprite "/Game/Textures/UI/Cell_Phone_Icon_Sprite_3.Cell_Phone_Icon_Sprite_3")
            (Variables|Default|SetFrame 0)))))))

(fn ConstructionScript)