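; DecisionUI is a VR actor that displays four decision options and five lines of text and tracks which option the player touches.
; BeginPlay records a start time and fills the text components from its string variables.
; Each of four colliders sets its own Decision boolean while the VRPawn overlaps it and clears it on exit.
; An EndDecision event destroys the actor.
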(event OnComponentEndOverlap(Collider4)
  (params (OverlappedComponent :type Primitive%20Component%20Object%20Reference) (OtherActor :type Actor%20Object%20Reference) (OtherComp :type Primitive%20Component%20Object%20Reference) (OtherBodyIndex :type Integer))
  (if (== (Utilities|GetClass OtherActor) "/Game/Blueprints/VRPawn.VRPawn_C")
    (Variables|Default|SetDecision4Bool false)))

(event OnComponentBeginOverlap(Collider1)
  (params (OverlappedComponent :type Primitive%20Component%20Object%20Reference) (OtherActor :type Actor%20Object%20Reference) (OtherComp :type Primitive%20Component%20Object%20Reference) (OtherBodyIndex :type Integer) (bFromSweep :type Boolean) (SweepResult :type Hit%20Result%20Structure%20%28by%20ref%29))
  (if (== (Utilities|GetClass OtherActor) "/Game/Blueprints/VRPawn.VRPawn_C")
    (Variables|Default|SetDecision1Bool true)))

(event OnComponentEndOverlap(Collider1)
  (params (OverlappedComponent :type Primitive%20Component%20Object%20Reference) (OtherActor :type Actor%20Object%20Reference) (OtherComp :type Primitive%20Component%20Object%20Reference) (OtherBodyIndex :type Integer))
  (if (== (Utilities|GetClass OtherActor) "/Game/Blueprints/VRPawn.VRPawn_C")
    (Variables|Default|SetDecision1Bool false)))

(event OnComponentBeginOverlap(Collider2)
  (params (OverlappedComponent :type Primitive%20Component%20Object%20Reference) (OtherActor :type Actor%20Object%20Reference) (OtherComp :type Primitive%20Component%20Object%20Reference) (OtherBodyIndex :type Integer) (bFromSweep :type Boolean) (SweepResult :type Hit%20Result%20Structure%20%28by%20ref%29))
  (if (== (Utilities|GetClass OtherActor) "/Game/Blueprints/VRPawn.VRPawn_C")
    (Variables|Default|SetDecision2Bool true)))

(event OnComponentEndOverlap(Collider2)
  (params (OverlappedComponent :type Primitive%20Component%20Object%20Reference) (OtherActor :type Actor%20Object%20Reference) (OtherComp :type Primitive%20Component%20Object%20Reference) (OtherBodyIndex :type Integer))
  (if (== (Utilities|GetClass OtherActor) "/Game/Blueprints/VRPawn.VRPawn_C")
    (Variables|Default|SetDecision2Bool false)))

(event OnComponentBeginOverlap(Collider3)
  (params (OverlappedComponent :type Primitive%20Component%20Object%20Reference) (OtherActor :type Actor%20Object%20Reference) (OtherComp :type Primitive%20Component%20Object%20Reference) (OtherBodyIndex :type Integer) (bFromSweep :type Boolean) (SweepResult :type Hit%20Result%20Structure%20%28by%20ref%29))
  (if (== (Utilities|GetClass OtherActor) "/Game/Blueprints/VRPawn.VRPawn_C")
    (Variables|Default|SetDecision3Bool true)))

(event OnComponentEndOverlap(Collider3)
  (params (OverlappedComponent :type Primitive%20Component%20Object%20Reference) (OtherActor :type Actor%20Object%20Reference) (OtherComp :type Primitive%20Component%20Object%20Reference) (OtherBodyIndex :type Integer))
  (if (== (Utilities|GetClass OtherActor) "/Game/Blueprints/VRPawn.VRPawn_C")
    (Variables|Default|SetDecision3Bool false)))

(event OnComponentBeginOverlap(Collider4)
  (params (OverlappedComponent :type Primitive%20Component%20Object%20Reference) (OtherActor :type Actor%20Object%20Reference) (OtherComp :type Primitive%20Component%20Object%20Reference) (OtherBodyIndex :type Integer) (bFromSweep :type Boolean) (SweepResult :type Hit%20Result%20Structure%20%28by%20ref%29))
  (if (== (Utilities|GetClass OtherActor) "/Game/Blueprints/VRPawn.VRPawn_C")
    (Variables|Default|SetDecision4Bool true)))

(event Custom|EndDecision
  (Actor|DestroyActor))

(event EventBeginPlay
  (Variables|Default|SetStartTime (Class|KismetStringLibrary|TimeSecondstoString (Utilities|Time|GetTimeSeconds)))
  (Rendering|Components|TextRender|SetText (Variables|Default|GetDecisionText1) (Utilities|Text|ToText(String) (Variables|Default|GetDecisionText)))
  (Rendering|Components|TextRender|SetText (Variables|Default|GetDecisionText2) (Utilities|Text|ToText(String) (Variables|Default|GetDecisionText_0)))
  (Rendering|Components|TextRender|SetText (Variables|Default|GetDecisionText3) (Utilities|Text|ToText(String) (Variables|Default|GetDecisionText_1)))
  (Rendering|Components|TextRender|SetText (Variables|Default|GetDecisionText4) (Utilities|Text|ToText(String) (Variables|Default|GetDecisionText_2)))
  (Rendering|Components|TextRender|SetText (Variables|Default|GetLine1) (Utilities|Text|ToText(String) (Variables|Default|GetlineText)))
  (Rendering|Components|TextRender|SetText (Variables|Default|GetLine2) (Utilities|Text|ToText(String) (Variables|Default|GetlineText_0)))
  (Rendering|Components|TextRender|SetText (Variables|Default|GetLine3) (Utilities|Text|ToText(String) (Variables|Default|GetlineText_1)))
  (Rendering|Components|TextRender|SetText (Variables|Default|GetLine4) (Utilities|Text|ToText(String) (Variables|Default|GetlineText_2)))
  (Rendering|Components|TextRender|SetText (Variables|Default|GetLine5) (Utilities|Text|ToText(String) (Variables|Default|GetlineText_3))))

(fn ConstructionScript)