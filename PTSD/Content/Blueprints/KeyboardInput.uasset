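; VR on-screen keyboard actor for entering the player's name before the game starts, also accepting physical key presses.
; Key overlaps set CurrentKeyOver, and Interact dispatches it to events that edit Name and its text display.
; Enter hides the keys, passes Name and Date to VRPawn, calls StartGame and destroys the actor; Done joins that path.
; A slash-formatting date numpad exists but is hidden at BeginPlay and absent from Interact.
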(event OnComponentBeginOverlap(Rb)
  (params (OverlappedComponent :type Primitive%20Component%20Object%20Reference) (OtherActor :type Actor%20Object%20Reference) (OtherComp :type Primitive%20Component%20Object%20Reference) (OtherBodyIndex :type Integer) (bFromSweep :type Boolean) (SweepResult :type Hit%20Result%20Structure%20%28by%20ref%29))
  ;[1 1 1] Keyboard collisions
  (Variables|Default|SetCurrentKeyOver "R"))

(event OnComponentBeginOverlap(Deltb)
  (params (OverlappedComponent :type Primitive%20Component%20Object%20Reference) (OtherActor :type Actor%20Object%20Reference) (OtherComp :type Primitive%20Component%20Object%20Reference) (OtherBodyIndex :type Integer) (bFromSweep :type Boolean) (SweepResult :type Hit%20Result%20Structure%20%28by%20ref%29))
  ;[1 1 1] Keyboard collisions
  (Variables|Default|SetCurrentKeyOver "-"))

(event OnComponentBeginOverlap(Sb)
  (params (OverlappedComponent :type Primitive%20Component%20Object%20Reference) (OtherActor :type Actor%20Object%20Reference) (OtherComp :type Primitive%20Component%20Object%20Reference) (OtherBodyIndex :type Integer) (bFromSweep :type Boolean) (SweepResult :type Hit%20Result%20Structure%20%28by%20ref%29))
  ;[1 1 1] Keyboard collisions
  (Variables|Default|SetCurrentKeyOver "S"))

(event OnComponentBeginOverlap(Qb)
  (params (OverlappedComponent :type Primitive%20Component%20Object%20Reference) (OtherActor :type Actor%20Object%20Reference) (OtherComp :type Primitive%20Component%20Object%20Reference) (OtherBodyIndex :type Integer) (bFromSweep :type Boolean) (SweepResult :type Hit%20Result%20Structure%20%28by%20ref%29))
  ;[1 1 1] Keyboard collisions
  (Variables|Default|SetCurrentKeyOver "Q"))

(event OnComponentBeginOverlap(Pb)
  (params (OverlappedComponent :type Primitive%20Component%20Object%20Reference) (OtherActor :type Actor%20Object%20Reference) (OtherComp :type Primitive%20Component%20Object%20Reference) (OtherBodyIndex :type Integer) (bFromSweep :type Boolean) (SweepResult :type Hit%20Result%20Structure%20%28by%20ref%29))
  ;[1 1 1] Keyboard collisions
  (Variables|Default|SetCurrentKeyOver "P"))

(event OnComponentBeginOverlap(Ob)
  (params (OverlappedComponent :type Primitive%20Component%20Object%20Reference) (OtherActor :type Actor%20Object%20Reference) (OtherComp :type Primitive%20Component%20Object%20Reference) (OtherBodyIndex :type Integer) (bFromSweep :type Boolean) (SweepResult :type Hit%20Result%20Structure%20%28by%20ref%29))
  ;[1 1 1] Keyboard collisions
  (Variables|Default|SetCurrentKeyOver "O"))

(event OnComponentBeginOverlap(Nb)
  (params (OverlappedComponent :type Primitive%20Component%20Object%20Reference) (OtherActor :type Actor%20Object%20Reference) (OtherComp :type Primitive%20Component%20Object%20Reference) (OtherBodyIndex :type Integer) (bFromSweep :type Boolean) (SweepResult :type Hit%20Result%20Structure%20%28by%20ref%29))
  ;[1 1 1] Keyboard collisions
  (Variables|Default|SetCurrentKeyOver "N"))

(event OnComponentBeginOverlap(Mb)
  (params (OverlappedComponent :type Primitive%20Component%20Object%20Reference) (OtherActor :type Actor%20Object%20Reference) (OtherComp :type Primitive%20Component%20Object%20Reference) (OtherBodyIndex :type Integer) (bFromSweep :type Boolean) (SweepResult :type Hit%20Result%20Structure%20%28by%20ref%29))
  ;[1 1 1] Keyboard collisions
  (Variables|Default|SetCurrentKeyOver "M"))

(event OnComponentBeginOverlap(Lb)
  (params (OverlappedComponent :type Primitive%20Component%20Object%20Reference) (OtherActor :type Actor%20Object%20Reference) (OtherComp :type Primitive%20Component%20Object%20Reference) (OtherBodyIndex :type Integer) (bFromSweep :type Boolean) (SweepResult :type Hit%20Result%20Structure%20%28by%20ref%29))
  ;[1 1 1] Keyboard collisions
  (Variables|Default|SetCurrentKeyOver "L"))

(event OnComponentBeginOverlap(KB)
  (params (OverlappedComponent :type Primitive%20Component%20Object%20Reference) (OtherActor :type Actor%20Object%20Reference) (OtherComp :type Primitive%20Component%20Object%20Reference) (OtherBodyIndex :type Integer) (bFromSweep :type Boolean) (SweepResult :type Hit%20Result%20Structure%20%28by%20ref%29))
  ;[1 1 1] Keyboard collisions
  (Variables|Default|SetCurrentKeyOver "K"))

(event OnComponentBeginOverlap(IB)
  (params (OverlappedComponent :type Primitive%20Component%20Object%20Reference) (OtherActor :type Actor%20Object%20Reference) (OtherComp :type Primitive%20Component%20Object%20Reference) (OtherBodyIndex :type Integer) (bFromSweep :type Boolean) (SweepResult :type Hit%20Result%20Structure%20%28by%20ref%29))
  ;[1 1 1] Keyboard collisions
  (Variables|Default|SetCurrentKeyOver "I"))

(event OnComponentBeginOverlap(Hb)
  (params (OverlappedComponent :type Primitive%20Component%20Object%20Reference) (OtherActor :type Actor%20Object%20Reference) (OtherComp :type Primitive%20Component%20Object%20Reference) (OtherBodyIndex :type Integer) (bFromSweep :type Boolean) (SweepResult :type Hit%20Result%20Structure%20%28by%20ref%29))
  ;[1 1 1] Keyboard collisions
  (Variables|Default|SetCurrentKeyOver "H"))

(event OnComponentBeginOverlap(Jb)
  (params (OverlappedComponent :type Primitive%20Component%20Object%20Reference) (OtherActor :type Actor%20Object%20Reference) (OtherComp :type Primitive%20Component%20Object%20Reference) (OtherBodyIndex :type Integer) (bFromSweep :type Boolean) (SweepResult :type Hit%20Result%20Structure%20%28by%20ref%29))
  ;[1 1 1] Keyboard collisions
  (Variables|Default|SetCurrentKeyOver "J"))

(event OnComponentBeginOverlap(Gb)
  (params (OverlappedComponent :type Primitive%20Component%20Object%20Reference) (OtherActor :type Actor%20Object%20Reference) (OtherComp :type Primitive%20Component%20Object%20Reference) (OtherBodyIndex :type Integer) (bFromSweep :type Boolean) (SweepResult :type Hit%20Result%20Structure%20%28by%20ref%29))
  ;[1 1 1] Keyboard collisions
  (Variables|Default|SetCurrentKeyOver "G"))

(event OnComponentBeginOverlap(0b)
  (params (OverlappedComponent :type Primitive%20Component%20Object%20Reference) (OtherActor :type Actor%20Object%20Reference) (OtherComp :type Primitive%20Component%20Object%20Reference) (OtherBodyIndex :type Integer) (bFromSweep :type Boolean) (SweepResult :type Hit%20Result%20Structure%20%28by%20ref%29))
  ;[1 1 1] Numberal Collisions
  (Variables|Default|SetCurrentKeyOver "0"))

(event OnComponentBeginOverlap(Fb)
  (params (OverlappedComponent :type Primitive%20Component%20Object%20Reference) (OtherActor :type Actor%20Object%20Reference) (OtherComp :type Primitive%20Component%20Object%20Reference) (OtherBodyIndex :type Integer) (bFromSweep :type Boolean) (SweepResult :type Hit%20Result%20Structure%20%28by%20ref%29))
  ;[1 1 1] Keyboard collisions
  (Variables|Default|SetCurrentKeyOver "F"))

(event OnComponentBeginOverlap(9b)
  (params (OverlappedComponent :type Primitive%20Component%20Object%20Reference) (OtherActor :type Actor%20Object%20Reference) (OtherComp :type Primitive%20Component%20Object%20Reference) (OtherBodyIndex :type Integer) (bFromSweep :type Boolean) (SweepResult :type Hit%20Result%20Structure%20%28by%20ref%29))
  ;[1 1 1] Numberal Collisions
  (Variables|Default|SetCurrentKeyOver "9"))

(event OnComponentBeginOverlap(8b)
  (params (OverlappedComponent :type Primitive%20Component%20Object%20Reference) (OtherActor :type Actor%20Object%20Reference) (OtherComp :type Primitive%20Component%20Object%20Reference) (OtherBodyIndex :type Integer) (bFromSweep :type Boolean) (SweepResult :type Hit%20Result%20Structure%20%28by%20ref%29))
  ;[1 1 1] Numberal Collisions
  (Variables|Default|SetCurrentKeyOver "8"))

(event OnComponentBeginOverlap(7b)
  (params (OverlappedComponent :type Primitive%20Component%20Object%20Reference) (OtherActor :type Actor%20Object%20Reference) (OtherComp :type Primitive%20Component%20Object%20Reference) (OtherBodyIndex :type Integer) (bFromSweep :type Boolean) (SweepResult :type Hit%20Result%20Structure%20%28by%20ref%29))
  ;[1 1 1] Numberal Collisions
  (Variables|Default|SetCurrentKeyOver "7"))

(event OnComponentBeginOverlap(Eb)
  (params (OverlappedComponent :type Primitive%20Component%20Object%20Reference) (OtherActor :type Actor%20Object%20Reference) (OtherComp :type Primitive%20Component%20Object%20Reference) (OtherBodyIndex :type Integer) (bFromSweep :type Boolean) (SweepResult :type Hit%20Result%20Structure%20%28by%20ref%29))
  ;[1 1 1] Keyboard collisions
  (Variables|Default|SetCurrentKeyOver "E"))

(event OnComponentBeginOverlap(6b)
  (params (OverlappedComponent :type Primitive%20Component%20Object%20Reference) (OtherActor :type Actor%20Object%20Reference) (OtherComp :type Primitive%20Component%20Object%20Reference) (OtherBodyIndex :type Integer) (bFromSweep :type Boolean) (SweepResult :type Hit%20Result%20Structure%20%28by%20ref%29))
  ;[1 1 1] Numberal Collisions
  (Variables|Default|SetCurrentKeyOver "6"))

(event OnComponentBeginOverlap(5b)
  (params (OverlappedComponent :type Primitive%20Component%20Object%20Reference) (OtherActor :type Actor%20Object%20Reference) (OtherComp :type Primitive%20Component%20Object%20Reference) (OtherBodyIndex :type Integer) (bFromSweep :type Boolean) (SweepResult :type Hit%20Result%20Structure%20%28by%20ref%29))
  ;[1 1 1] Numberal Collisions
  (Variables|Default|SetCurrentKeyOver "5"))

(event OnComponentBeginOverlap(4b)
  (params (OverlappedComponent :type Primitive%20Component%20Object%20Reference) (OtherActor :type Actor%20Object%20Reference) (OtherComp :type Primitive%20Component%20Object%20Reference) (OtherBodyIndex :type Integer) (bFromSweep :type Boolean) (SweepResult :type Hit%20Result%20Structure%20%28by%20ref%29))
  ;[1 1 1] Numberal Collisions
  (Variables|Default|SetCurrentKeyOver "4"))

(event OnComponentBeginOverlap(DB)
  (params (OverlappedComponent :type Primitive%20Component%20Object%20Reference) (OtherActor :type Actor%20Object%20Reference) (OtherComp :type Primitive%20Component%20Object%20Reference) (OtherBodyIndex :type Integer) (bFromSweep :type Boolean) (SweepResult :type Hit%20Result%20Structure%20%28by%20ref%29))
  ;[1 1 1] Keyboard collisions
  (Variables|Default|SetCurrentKeyOver "D"))

(event OnComponentBeginOverlap(3b)
  (params (OverlappedComponent :type Primitive%20Component%20Object%20Reference) (OtherActor :type Actor%20Object%20Reference) (OtherComp :type Primitive%20Component%20Object%20Reference) (OtherBodyIndex :type Integer) (bFromSweep :type Boolean) (SweepResult :type Hit%20Result%20Structure%20%28by%20ref%29))
  ;[1 1 1] Numberal Collisions
  (Variables|Default|SetCurrentKeyOver "3"))

(event OnComponentBeginOverlap(2b)
  (params (OverlappedComponent :type Primitive%20Component%20Object%20Reference) (OtherActor :type Actor%20Object%20Reference) (OtherComp :type Primitive%20Component%20Object%20Reference) (OtherBodyIndex :type Integer) (bFromSweep :type Boolean) (SweepResult :type Hit%20Result%20Structure%20%28by%20ref%29))
  ;[1 1 1] Numberal Collisions
  (Variables|Default|SetCurrentKeyOver "2"))

(event OnComponentBeginOverlap(Cb)
  (params (OverlappedComponent :type Primitive%20Component%20Object%20Reference) (OtherActor :type Actor%20Object%20Reference) (OtherComp :type Primitive%20Component%20Object%20Reference) (OtherBodyIndex :type Integer) (bFromSweep :type Boolean) (SweepResult :type Hit%20Result%20Structure%20%28by%20ref%29))
  ;[1 1 1] Keyboard collisions
  (Variables|Default|SetCurrentKeyOver "C"))

(event OnComponentBeginOverlap(1b)
  (params (OverlappedComponent :type Primitive%20Component%20Object%20Reference) (OtherActor :type Actor%20Object%20Reference) (OtherComp :type Primitive%20Component%20Object%20Reference) (OtherBodyIndex :type Integer) (bFromSweep :type Boolean) (SweepResult :type Hit%20Result%20Structure%20%28by%20ref%29))
  ;[1 1 1] Numberal Collisions
  (Variables|Default|SetCurrentKeyOver "1"))

(event OnComponentBeginOverlap(Doneb)
  (params (OverlappedComponent :type Primitive%20Component%20Object%20Reference) (OtherActor :type Actor%20Object%20Reference) (OtherComp :type Primitive%20Component%20Object%20Reference) (OtherBodyIndex :type Integer) (bFromSweep :type Boolean) (SweepResult :type Hit%20Result%20Structure%20%28by%20ref%29))
  ;[1 1 1] Keyboard collisions
  (Variables|Default|SetCurrentKeyOver "Done"))

(event OnComponentBeginOverlap(Ndelb)
  (params (OverlappedComponent :type Primitive%20Component%20Object%20Reference) (OtherActor :type Actor%20Object%20Reference) (OtherComp :type Primitive%20Component%20Object%20Reference) (OtherBodyIndex :type Integer) (bFromSweep :type Boolean) (SweepResult :type Hit%20Result%20Structure%20%28by%20ref%29))
  ;[1 1 1] Numberal Collisions
  (Variables|Default|SetCurrentKeyOver "Ndel"))

(event OnComponentBeginOverlap(bb)
  (params (OverlappedComponent :type Primitive%20Component%20Object%20Reference) (OtherActor :type Actor%20Object%20Reference) (OtherComp :type Primitive%20Component%20Object%20Reference) (OtherBodyIndex :type Integer) (bFromSweep :type Boolean) (SweepResult :type Hit%20Result%20Structure%20%28by%20ref%29))
  ;[1 1 1] Keyboard collisions
  (Variables|Default|SetCurrentKeyOver "B"))

(event OnComponentBeginOverlap(ab)
  (params (OverlappedComponent :type Primitive%20Component%20Object%20Reference) (OtherActor :type Actor%20Object%20Reference) (OtherComp :type Primitive%20Component%20Object%20Reference) (OtherBodyIndex :type Integer) (bFromSweep :type Boolean) (SweepResult :type Hit%20Result%20Structure%20%28by%20ref%29))
  ;[1 1 1] Keyboard collisions
  (Variables|Default|SetCurrentKeyOver "A"))

(event OnComponentBeginOverlap(Zb)
  (params (OverlappedComponent :type Primitive%20Component%20Object%20Reference) (OtherActor :type Actor%20Object%20Reference) (OtherComp :type Primitive%20Component%20Object%20Reference) (OtherBodyIndex :type Integer) (bFromSweep :type Boolean) (SweepResult :type Hit%20Result%20Structure%20%28by%20ref%29))
  ;[1 1 1] Keyboard collisions
  (Variables|Default|SetCurrentKeyOver "Z"))

(event OnComponentBeginOverlap(yb)
  (params (OverlappedComponent :type Primitive%20Component%20Object%20Reference) (OtherActor :type Actor%20Object%20Reference) (OtherComp :type Primitive%20Component%20Object%20Reference) (OtherBodyIndex :type Integer) (bFromSweep :type Boolean) (SweepResult :type Hit%20Result%20Structure%20%28by%20ref%29))
  ;[1 1 1] Keyboard collisions
  (Variables|Default|SetCurrentKeyOver "Y"))

(event OnComponentBeginOverlap(Xb)
  (params (OverlappedComponent :type Primitive%20Component%20Object%20Reference) (OtherActor :type Actor%20Object%20Reference) (OtherComp :type Primitive%20Component%20Object%20Reference) (OtherBodyIndex :type Integer) (bFromSweep :type Boolean) (SweepResult :type Hit%20Result%20Structure%20%28by%20ref%29))
  ;[1 1 1] Keyboard collisions
  (Variables|Default|SetCurrentKeyOver "X"))

(event OnComponentBeginOverlap(Wb)
  (params (OverlappedComponent :type Primitive%20Component%20Object%20Reference) (OtherActor :type Actor%20Object%20Reference) (OtherComp :type Primitive%20Component%20Object%20Reference) (OtherBodyIndex :type Integer) (bFromSweep :type Boolean) (SweepResult :type Hit%20Result%20Structure%20%28by%20ref%29))
  ;[1 1 1] Keyboard collisions
  (Variables|Default|SetCurrentKeyOver "W"))

(event OnComponentBeginOverlap(vb)
  (params (OverlappedComponent :type Primitive%20Component%20Object%20Reference) (OtherActor :type Actor%20Object%20Reference) (OtherComp :type Primitive%20Component%20Object%20Reference) (OtherBodyIndex :type Integer) (bFromSweep :type Boolean) (SweepResult :type Hit%20Result%20Structure%20%28by%20ref%29))
  ;[1 1 1] Keyboard collisions
  (Variables|Default|SetCurrentKeyOver "V"))

(event OnComponentBeginOverlap(ub)
  (params (OverlappedComponent :type Primitive%20Component%20Object%20Reference) (OtherActor :type Actor%20Object%20Reference) (OtherComp :type Primitive%20Component%20Object%20Reference) (OtherBodyIndex :type Integer) (bFromSweep :type Boolean) (SweepResult :type Hit%20Result%20Structure%20%28by%20ref%29))
  ;[1 1 1] Keyboard collisions
  (Variables|Default|SetCurrentKeyOver "U"))

(event OnComponentBeginOverlap(Tb)
  (params (OverlappedComponent :type Primitive%20Component%20Object%20Reference) (OtherActor :type Actor%20Object%20Reference) (OtherComp :type Primitive%20Component%20Object%20Reference) (OtherBodyIndex :type Integer) (bFromSweep :type Boolean) (SweepResult :type Hit%20Result%20Structure%20%28by%20ref%29))
  ;[1 1 1] Keyboard collisions
  (Variables|Default|SetCurrentKeyOver "T"))

(event Custom|Interact
  (switch string (Variables|Default|GetCurrentKeyOver)
    (:A
      (CallFunction|Ae))
    (:B
      (CallFunction|Be))
    (:C
      (CallFunction|Ce))
    (:D
      (CallFunction|De))
    (:E
      (CallFunction|Ee))
    (:F
      (CallFunction|Fe))
    (:G
      (CallFunction|Ge))
    (:H
      (CallFunction|He))
    (:I
      (CallFunction|Ie))
    (:J
      (CallFunction|Je))
    (:K
      (CallFunction|Ke))
    (:L
      (CallFunction|Le))
    (:M
      (CallFunction|Me))
    (:N
      (CallFunction|Ne))
    (:O
      (CallFunction|Oe))
    (:P
      (CallFunction|Pe))
    (:Q
      (CallFunction|Qe))
    (:R
      (CallFunction|Re))
    (:S
      (CallFunction|Se))
    (:T
      (CallFunction|Te))
    (:U
      (CallFunction|Ue))
    (:V
      (CallFunction|Ve))
    (:W
      (CallFunction|We))
    (:X
      (CallFunction|Xe))
    (:Y
      (CallFunction|Ye))
    (:Z
      (CallFunction|Ze))
    (:-
      (CallFunction|Dele))
    (:Done
      (CallFunction|DoneEvent))))

(event Custom|Fe
  ;[1 1 1] Keyboard Events
  (bind _output_get (Variables|Default|SetName (Utilities|String|Append (Variables|Default|GetName) "F")))
  (Rendering|Components|TextRender|SetText (Variables|Default|GetNameT) (Utilities|Text|ToText(String) _output_get)))

(event Custom|Ge
  ;[1 1 1] Keyboard Events
  (bind _output_get (Variables|Default|SetName (Utilities|String|Append (Variables|Default|GetName) "G")))
  (Rendering|Components|TextRender|SetText (Variables|Default|GetNameT) (Utilities|Text|ToText(String) _output_get)))

(event Custom|He
  ;[1 1 1] Keyboard Events
  (bind _output_get (Variables|Default|SetName (Utilities|String|Append (Variables|Default|GetName) "H")))
  (Rendering|Components|TextRender|SetText (Variables|Default|GetNameT) (Utilities|Text|ToText(String) _output_get)))

(event Custom|Ie
  ;[1 1 1] Keyboard Events
  (bind _output_get (Variables|Default|SetName (Utilities|String|Append (Variables|Default|GetName) "I")))
  (Rendering|Components|TextRender|SetText (Variables|Default|GetNameT) (Utilities|Text|ToText(String) _output_get)))

(event Custom|Je
  ;[1 1 1] Keyboard Events
  (bind _output_get (Variables|Default|SetName (Utilities|String|Append (Variables|Default|GetName) "J")))
  (Rendering|Components|TextRender|SetText (Variables|Default|GetNameT) (Utilities|Text|ToText(String) _output_get)))

(event Custom|7e
  ;[1 1 1] Numberal Events
  (Variables|Default|SetDate (Utilities|String|Append (Variables|Default|GetDate) "7"))
  (if (== (Utilities|String|Len (Variables|Default|GetDate)) 2)
    (Variables|Default|SetDate (Utilities|String|Append (Variables|Default|GetDate) "/") :!label _label)
    (elif (== (Utilities|String|Len (Variables|Default|GetDate)) 5)
      (goto _label)
      (elif (> (Utilities|String|Len (Variables|Default|GetDate)) 8)
        (Variables|Default|SetDate (Utilities|String|LeftChop (Variables|Default|GetDate) 1)))))
  (Rendering|Components|TextRender|SetText (Variables|Default|GetDateT) (Utilities|Text|ToText(String) (Variables|Default|GetDate))))

(event Custom|8e
  ;[1 1 1] Numberal Events
  (Variables|Default|SetDate (Utilities|String|Append (Variables|Default|GetDate) "8"))
  (if (== (Utilities|String|Len (Variables|Default|GetDate)) 2)
    (Variables|Default|SetDate (Utilities|String|Append (Variables|Default|GetDate) "/") :!label _label)
    (elif (== (Utilities|String|Len (Variables|Default|GetDate)) 5)
      (goto _label)
      (elif (> (Utilities|String|Len (Variables|Default|GetDate)) 8)
        (Variables|Default|SetDate (Utilities|String|LeftChop (Variables|Default|GetDate) 1)))))
  (Rendering|Components|TextRender|SetText (Variables|Default|GetDateT) (Utilities|Text|ToText(String) (Variables|Default|GetDate))))

(event Custom|Ve
  ;[1 1 1] Keyboard Events
  (bind _output_get (Variables|Default|SetName (Utilities|String|Append (Variables|Default|GetName) "V")))
  (Rendering|Components|TextRender|SetText (Variables|Default|GetNameT) (Utilities|Text|ToText(String) _output_get)))

(event Custom|We
  ;[1 1 1] Keyboard Events
  (bind _output_get (Variables|Default|SetName (Utilities|String|Append (Variables|Default|GetName) "W")))
  (Rendering|Components|TextRender|SetText (Variables|Default|GetNameT) (Utilities|Text|ToText(String) _output_get)))

(event Custom|Xe
  ;[1 1 1] Keyboard Events
  (bind _output_get (Variables|Default|SetName (Utilities|String|Append (Variables|Default|GetName) "X")))
  (Rendering|Components|TextRender|SetText (Variables|Default|GetNameT) (Utilities|Text|ToText(String) _output_get)))

(event Custom|Ye
  ;[1 1 1] Keyboard Events
  (bind _output_get (Variables|Default|SetName (Utilities|String|Append (Variables|Default|GetName) "Y")))
  (Rendering|Components|TextRender|SetText (Variables|Default|GetNameT) (Utilities|Text|ToText(String) _output_get)))

(event Custom|Ze
  ;[1 1 1] Keyboard Events
  (bind _output_get (Variables|Default|SetName (Utilities|String|Append (Variables|Default|GetName) "Z")))
  (Rendering|Components|TextRender|SetText (Variables|Default|GetNameT) (Utilities|Text|ToText(String) _output_get)))

(event Custom|Dele
  ;[1 1 1] Keyboard Events
  (bind _output_get (Variables|Default|SetName (Utilities|String|LeftChop (Variables|Default|GetName) 1)))
  (Rendering|Components|TextRender|SetText (Variables|Default|GetNameT) (Utilities|Text|ToText(String) _output_get)))

(event Custom|DoneEvent
  (for _array_element (Components|GetChildrenComponents (Variables|Default|GetKeyBoard) true)
    (Rendering|SetVisibility _array_element false true))
  (bind _asvrpawn (Utilities|Casting|CastToVRPawn (Game|Player|GetPlayerPawn 0)))
  (Variables|/Game/Blueprints/VRPawn.VRPawn_C|SetName _asvrpawn (Variables|Default|GetName))
  (Variables|/Game/Blueprints/VRPawn.VRPawn_C|SetDate _asvrpawn (Variables|Default|GetDate))
  (Default|StartGame _asvrpawn)
  (Actor|DestroyActor))

(event Custom|1e
  ;[1 1 1] Numberal Events
  (Variables|Default|SetDate (Utilities|String|Append (Variables|Default|GetDate) "1"))
  (if (== (Utilities|String|Len (Variables|Default|GetDate)) 2)
    (Variables|Default|SetDate (Utilities|String|Append (Variables|Default|GetDate) "/") :!label _label)
    (elif (== (Utilities|String|Len (Variables|Default|GetDate)) 5)
      (goto _label)
      (elif (> (Utilities|String|Len (Variables|Default|GetDate)) 8)
        (Variables|Default|SetDate (Utilities|String|LeftChop (Variables|Default|GetDate) 1)))))
  (Rendering|Components|TextRender|SetText (Variables|Default|GetDateT) (Utilities|Text|ToText(String) (Variables|Default|GetDate))))

(event Custom|2e
  ;[1 1 1] Numberal Events
  (Variables|Default|SetDate (Utilities|String|Append (Variables|Default|GetDate) "2"))
  (if (== (Utilities|String|Len (Variables|Default|GetDate)) 2)
    (Variables|Default|SetDate (Utilities|String|Append (Variables|Default|GetDate) "/") :!label _label)
    (elif (== (Utilities|String|Len (Variables|Default|GetDate)) 5)
      (goto _label)
      (elif (> (Utilities|String|Len (Variables|Default|GetDate)) 8)
        (Variables|Default|SetDate (Utilities|String|LeftChop (Variables|Default|GetDate) 1)))))
  (Rendering|Components|TextRender|SetText (Variables|Default|GetDateT) (Utilities|Text|ToText(String) (Variables|Default|GetDate))))

(event Custom|3e
  ;[1 1 1] Numberal Events
  (Variables|Default|SetDate (Utilities|String|Append (Variables|Default|GetDate) "3"))
  (if (== (Utilities|String|Len (Variables|Default|GetDate)) 2)
    (Variables|Default|SetDate (Utilities|String|Append (Variables|Default|GetDate) "/") :!label _label)
    (elif (== (Utilities|String|Len (Variables|Default|GetDate)) 5)
      (goto _label)
      (elif (> (Utilities|String|Len (Variables|Default|GetDate)) 8)
        (Variables|Default|SetDate (Utilities|String|LeftChop (Variables|Default|GetDate) 1)))))
  (Rendering|Components|TextRender|SetText (Variables|Default|GetDateT) (Utilities|Text|ToText(String) (Variables|Default|GetDate))))

(event Custom|4e
  ;[1 1 1] Numberal Events
  (Variables|Default|SetDate (Utilities|String|Append (Variables|Default|GetDate) "4"))
  (if (== (Utilities|String|Len (Variables|Default|GetDate)) 2)
    (Variables|Default|SetDate (Utilities|String|Append (Variables|Default|GetDate) "/") :!label _label)
    (elif (== (Utilities|String|Len (Variables|Default|GetDate)) 5)
      (goto _label)
      (elif (> (Utilities|String|Len (Variables|Default|GetDate)) 8)
        (Variables|Default|SetDate (Utilities|String|LeftChop (Variables|Default|GetDate) 1)))))
  (Rendering|Components|TextRender|SetText (Variables|Default|GetDateT) (Utilities|Text|ToText(String) (Variables|Default|GetDate))))

(event Custom|5e
  ;[1 1 1] Numberal Events
  (Variables|Default|SetDate (Utilities|String|Append (Variables|Default|GetDate) "5"))
  (if (== (Utilities|String|Len (Variables|Default|GetDate)) 2)
    (Variables|Default|SetDate (Utilities|String|Append (Variables|Default|GetDate) "/") :!label _label)
    (elif (== (Utilities|String|Len (Variables|Default|GetDate)) 5)
      (goto _label)
      (elif (> (Utilities|String|Len (Variables|Default|GetDate)) 8)
        (Variables|Default|SetDate (Utilities|String|LeftChop (Variables|Default|GetDate) 1)))))
  (Rendering|Components|TextRender|SetText (Variables|Default|GetDateT) (Utilities|Text|ToText(String) (Variables|Default|GetDate))))

(event Custom|0e
  ;[1 1 1] Numberal Events
  (Variables|Default|SetDate (Utilities|String|Append (Variables|Default|GetDate) "0"))
  (if (== (Utilities|String|Len (Variables|Default|GetDate)) 2)
    (Variables|Default|SetDate (Utilities|String|Append (Variables|Default|GetDate) "/") :!label _label)
    (elif (== (Utilities|String|Len (Variables|Default|GetDate)) 5)
      (goto _label)
      (elif (> (Utilities|String|Len (Variables|Default|GetDate)) 8)
        (Variables|Default|SetDate (Utilities|String|LeftChop (Variables|Default|GetDate) 1)))))
  (Rendering|Components|TextRender|SetText (Variables|Default|GetDateT) (Utilities|Text|ToText(String) (Variables|Default|GetDate))))

(event Custom|Ke
  ;[1 1 1] Keyboard Events
  (bind _output_get (Variables|Default|SetName (Utilities|String|Append (Variables|Default|GetName) "K")))
  (Rendering|Components|TextRender|SetText (Variables|Default|GetNameT) (Utilities|Text|ToText(String) _output_get)))

(event Custom|Le
  ;[1 1 1] Keyboard Events
  (bind _output_get (Variables|Default|SetName (Utilities|String|Append (Variables|Default|GetName) "L")))
  (Rendering|Components|TextRender|SetText (Variables|Default|GetNameT) (Utilities|Text|ToText(String) _output_get)))

(event Custom|Me
  ;[1 1 1] Keyboard Events
  (bind _output_get (Variables|Default|SetName (Utilities|String|Append (Variables|Default|GetName) "M")))
  (Rendering|Components|TextRender|SetText (Variables|Default|GetNameT) (Utilities|Text|ToText(String) _output_get)))

(event Custom|Ne
  ;[1 1 1] Keyboard Events
  (bind _output_get (Variables|Default|SetName (Utilities|String|Append (Variables|Default|GetName) "N")))
  (Rendering|Components|TextRender|SetText (Variables|Default|GetNameT) (Utilities|Text|ToText(String) _output_get)))

(event Custom|Oe
  ;[1 1 1] Keyboard Events
  (bind _output_get (Variables|Default|SetName (Utilities|String|Append (Variables|Default|GetName) "O")))
  (Rendering|Components|TextRender|SetText (Variables|Default|GetNameT) (Utilities|Text|ToText(String) _output_get)))

(event Custom|6e
  ;[1 1 1] Numberal Events
  (Variables|Default|SetDate (Utilities|String|Append (Variables|Default|GetDate) "6"))
  (if (== (Utilities|String|Len (Variables|Default|GetDate)) 2)
    (Variables|Default|SetDate (Utilities|String|Append (Variables|Default|GetDate) "/") :!label _label)
    (elif (== (Utilities|String|Len (Variables|Default|GetDate)) 5)
      (goto _label)
      (elif (> (Utilities|String|Len (Variables|Default|GetDate)) 8)
        (Variables|Default|SetDate (Utilities|String|LeftChop (Variables|Default|GetDate) 1)))))
  (Rendering|Components|TextRender|SetText (Variables|Default|GetDateT) (Utilities|Text|ToText(String) (Variables|Default|GetDate))))

(event Custom|Re
  ;[1 1 1] Keyboard Events
  (bind _output_get (Variables|Default|SetName (Utilities|String|Append (Variables|Default|GetName) "R")))
  (Rendering|Components|TextRender|SetText (Variables|Default|GetNameT) (Utilities|Text|ToText(String) _output_get)))

(event Custom|Se
  ;[1 1 1] Keyboard Events
  (bind _output_get (Variables|Default|SetName (Utilities|String|Append (Variables|Default|GetName) "S")))
  (Rendering|Components|TextRender|SetText (Variables|Default|GetNameT) (Utilities|Text|ToText(String) _output_get)))

(event Custom|Te
  ;[1 1 1] Keyboard Events
  (bind _output_get (Variables|Default|SetName (Utilities|String|Append (Variables|Default|GetName) "T")))
  (Rendering|Components|TextRender|SetText (Variables|Default|GetNameT) (Utilities|Text|ToText(String) _output_get)))

(event Custom|Ue
  ;[1 1 1] Keyboard Events
  (bind _output_get (Variables|Default|SetName (Utilities|String|Append (Variables|Default|GetName) "U")))
  (Rendering|Components|TextRender|SetText (Variables|Default|GetNameT) (Utilities|Text|ToText(String) _output_get)))

(event Custom|9e
  ;[1 1 1] Numberal Events
  (Variables|Default|SetDate (Utilities|String|Append (Variables|Default|GetDate) "9"))
  (if (== (Utilities|String|Len (Variables|Default|GetDate)) 2)
    (Variables|Default|SetDate (Utilities|String|Append (Variables|Default|GetDate) "/") :!label _label)
    (elif (== (Utilities|String|Len (Variables|Default|GetDate)) 5)
      (goto _label)
      (elif (> (Utilities|String|Len (Variables|Default|GetDate)) 8)
        (Variables|Default|SetDate (Utilities|String|LeftChop (Variables|Default|GetDate) 1)))))
  (Rendering|Components|TextRender|SetText (Variables|Default|GetDateT) (Utilities|Text|ToText(String) (Variables|Default|GetDate))))

(event Custom|nDele
  ;[1 1 1] Numberal Events
  (Variables|Default|SetDate (Utilities|String|LeftChop (Variables|Default|GetDate) 1))
  (Rendering|Components|TextRender|SetText (Variables|Default|GetDateT) (Utilities|Text|ToText(String) (Variables|Default|GetDate))))

(event Custom|Qe
  ;[1 1 1] Keyboard Events
  (bind _output_get (Variables|Default|SetName (Utilities|String|Append (Variables|Default|GetName) "Q")))
  (Rendering|Components|TextRender|SetText (Variables|Default|GetNameT) (Utilities|Text|ToText(String) _output_get)))

(event Custom|Pe
  ;[1 1 1] Keyboard Events
  (bind _output_get (Variables|Default|SetName (Utilities|String|Append (Variables|Default|GetName) "P")))
  (Rendering|Components|TextRender|SetText (Variables|Default|GetNameT) (Utilities|Text|ToText(String) _output_get)))

(event Custom|Ae
  ;[1 1 1] Keyboard Events
  (bind _output_get (Variables|Default|SetName (Utilities|String|Append (Variables|Default|GetName) "A")))
  (Rendering|Components|TextRender|SetText (Variables|Default|GetNameT) (Utilities|Text|ToText(String) _output_get)))

(event Custom|Be
  ;[1 1 1] Keyboard Events
  (bind _output_get (Variables|Default|SetName (Utilities|String|Append (Variables|Default|GetName) "B")))
  (Rendering|Components|TextRender|SetText (Variables|Default|GetNameT) (Utilities|Text|ToText(String) _output_get)))

(event Custom|Ce
  ;[1 1 1] Keyboard Events
  (bind _output_get (Variables|Default|SetName (Utilities|String|Append (Variables|Default|GetName) "C")))
  (Rendering|Components|TextRender|SetText (Variables|Default|GetNameT) (Utilities|Text|ToText(String) _output_get)))

(event Custom|De
  ;[1 1 1] Keyboard Events
  (bind _output_get (Variables|Default|SetName (Utilities|String|Append (Variables|Default|GetName) "D")))
  (Rendering|Components|TextRender|SetText (Variables|Default|GetNameT) (Utilities|Text|ToText(String) _output_get)))

(event Custom|Ee
  ;[1 1 1] Keyboard Events
  (bind _output_get (Variables|Default|SetName (Utilities|String|Append (Variables|Default|GetName) "E")))
  (Rendering|Components|TextRender|SetText (Variables|Default|GetNameT) (Utilities|Text|ToText(String) _output_get)))

(event EventBeginPlay
  (for _array_element (Components|GetChildrenComponents (Variables|Default|GetNumberal) false)
    (Rendering|SetVisibility _array_element false true)))

(event Input|KeyboardEvents|V
  (params (Key :type Key%20Structure :default "AnyKey"))
  ;[1 1 1] Keyboard Events
  (:Pressed
    (bind _output_get (Variables|Default|SetName (Utilities|String|Append (Variables|Default|GetName) "V")))
    (Rendering|Components|TextRender|SetText (Variables|Default|GetNameT) (Utilities|Text|ToText(String) _output_get))))

(event Input|KeyboardEvents|Z
  (params (Key :type Key%20Structure :default "AnyKey"))
  ;[1 1 1] Keyboard Events
  (:Pressed
    (bind _output_get (Variables|Default|SetName (Utilities|String|Append (Variables|Default|GetName) "Z")))
    (Rendering|Components|TextRender|SetText (Variables|Default|GetNameT) (Utilities|Text|ToText(String) _output_get))))

(event Input|KeyboardEvents|Backspace
  (params (Key :type Key%20Structure :default "AnyKey"))
  ;[1 1 1] Keyboard Events
  (:Pressed
    (bind _output_get (Variables|Default|SetName (Utilities|String|LeftChop (Variables|Default|GetName) 1)))
    (Rendering|Components|TextRender|SetText (Variables|Default|GetNameT) (Utilities|Text|ToText(String) _output_get))))

(event Input|KeyboardEvents|W
  (params (Key :type Key%20Structure :default "AnyKey"))
  ;[1 1 1] Keyboard Events
  (:Pressed
    (bind _output_get (Variables|Default|SetName (Utilities|String|Append (Variables|Default|GetName) "W")))
    (Rendering|Components|TextRender|SetText (Variables|Default|GetNameT) (Utilities|Text|ToText(String) _output_get))))

(event Input|KeyboardEvents|X
  (params (Key :type Key%20Structure :default "AnyKey"))
  ;[1 1 1] Keyboard Events
  (:Pressed
    (bind _output_get (Variables|Default|SetName (Utilities|String|Append (Variables|Default|GetName) "X")))
    (Rendering|Components|TextRender|SetText (Variables|Default|GetNameT) (Utilities|Text|ToText(String) _output_get))))

(event Input|KeyboardEvents|P
  (params (Key :type Key%20Structure :default "AnyKey"))
  ;[1 1 1] Keyboard Events
  (:Pressed
    (bind _output_get (Variables|Default|SetName (Utilities|String|Append (Variables|Default|GetName) "P")))
    (Rendering|Components|TextRender|SetText (Variables|Default|GetNameT) (Utilities|Text|ToText(String) _output_get))))

(event Input|KeyboardEvents|Y
  (params (Key :type Key%20Structure :default "AnyKey"))
  ;[1 1 1] Keyboard Events
  (:Pressed
    (bind _output_get (Variables|Default|SetName (Utilities|String|Append (Variables|Default|GetName) "Y")))
    (Rendering|Components|TextRender|SetText (Variables|Default|GetNameT) (Utilities|Text|ToText(String) _output_get))))

(event Input|KeyboardEvents|A
  (params (Key :type Key%20Structure :default "AnyKey"))
  ;[1 1 1] Keyboard Events
  (:Pressed
    (bind _output_get (Variables|Default|SetName (Utilities|String|Append (Variables|Default|GetName) "A")))
    (Rendering|Components|TextRender|SetText (Variables|Default|GetNameT) (Utilities|Text|ToText(String) _output_get))))

(event Input|KeyboardEvents|B
  (params (Key :type Key%20Structure :default "AnyKey"))
  ;[1 1 1] Keyboard Events
  (:Pressed
    (bind _output_get (Variables|Default|SetName (Utilities|String|Append (Variables|Default|GetName) "B")))
    (Rendering|Components|TextRender|SetText (Variables|Default|GetNameT) (Utilities|Text|ToText(String) _output_get))))

(event Input|KeyboardEvents|Enter
  (params (Key :type Key%20Structure :default "AnyKey"))
  (:Pressed
    (Utilities|FlowControl|FlipFlop
      (:A
        (for _array_element (Components|GetChildrenComponents (Variables|Default|GetKeyBoard) true)
          (Rendering|SetVisibility _array_element false true)))
      (:B
        _))
    (bind _asvrpawn (Utilities|Casting|CastToVRPawn (Game|Player|GetPlayerPawn 0)))
    (Variables|/Game/Blueprints/VRPawn.VRPawn_C|SetName _asvrpawn (Variables|Default|GetName))
    (Variables|/Game/Blueprints/VRPawn.VRPawn_C|SetDate _asvrpawn (Variables|Default|GetDate))
    (Default|StartGame _asvrpawn)
    (Actor|DestroyActor)))

(event Input|KeyboardEvents|C
  (params (Key :type Key%20Structure :default "AnyKey"))
  ;[1 1 1] Keyboard Events
  (:Pressed
    (bind _output_get (Variables|Default|SetName (Utilities|String|Append (Variables|Default|GetName) "C")))
    (Rendering|Components|TextRender|SetText (Variables|Default|GetNameT) (Utilities|Text|ToText(String) _output_get))))

(event Input|KeyboardEvents|D
  (params (Key :type Key%20Structure :default "AnyKey"))
  ;[1 1 1] Keyboard Events
  (:Pressed
    (bind _output_get (Variables|Default|SetName (Utilities|String|Append (Variables|Default|GetName) "D")))
    (Rendering|Components|TextRender|SetText (Variables|Default|GetNameT) (Utilities|Text|ToText(String) _output_get))))

(event Input|KeyboardEvents|E
  (params (Key :type Key%20Structure :default "AnyKey"))
  ;[1 1 1] Keyboard Events
  (:Pressed
    (bind _output_get (Variables|Default|SetName (Utilities|String|Append (Variables|Default|GetName) "E")))
    (Rendering|Components|TextRender|SetText (Variables|Default|GetNameT) (Utilities|Text|ToText(String) _output_get))))

(event Input|KeyboardEvents|F
  (params (Key :type Key%20Structure :default "AnyKey"))
  ;[1 1 1] Keyboard Events
  (:Pressed
    (bind _output_get (Variables|Default|SetName (Utilities|String|Append (Variables|Default|GetName) "F")))
    (Rendering|Components|TextRender|SetText (Variables|Default|GetNameT) (Utilities|Text|ToText(String) _output_get))))

(event Input|KeyboardEvents|G
  (params (Key :type Key%20Structure :default "AnyKey"))
  ;[1 1 1] Keyboard Events
  (:Pressed
    (bind _output_get (Variables|Default|SetName (Utilities|String|Append (Variables|Default|GetName) "G")))
    (Rendering|Components|TextRender|SetText (Variables|Default|GetNameT) (Utilities|Text|ToText(String) _output_get))))

(event Input|KeyboardEvents|H
  (params (Key :type Key%20Structure :default "AnyKey"))
  ;[1 1 1] Keyboard Events
  (:Pressed
    (bind _output_get (Variables|Default|SetName (Utilities|String|Append (Variables|Default|GetName) "H")))
    (Rendering|Components|TextRender|SetText (Variables|Default|GetNameT) (Utilities|Text|ToText(String) _output_get))))

(event Input|KeyboardEvents|I
  (params (Key :type Key%20Structure :default "AnyKey"))
  ;[1 1 1] Keyboard Events
  (:Pressed
    (bind _output_get (Variables|Default|SetName (Utilities|String|Append (Variables|Default|GetName) "I")))
    (Rendering|Components|TextRender|SetText (Variables|Default|GetNameT) (Utilities|Text|ToText(String) _output_get))))

(event Input|KeyboardEvents|J
  (params (Key :type Key%20Structure :default "AnyKey"))
  ;[1 1 1] Keyboard Events
  (:Pressed
    (bind _output_get (Variables|Default|SetName (Utilities|String|Append (Variables|Default|GetName) "J")))
    (Rendering|Components|TextRender|SetText (Variables|Default|GetNameT) (Utilities|Text|ToText(String) _output_get))))

(event Input|KeyboardEvents|K
  (params (Key :type Key%20Structure :default "AnyKey"))
  ;[1 1 1] Keyboard Events
  (:Pressed
    (bind _output_get (Variables|Default|SetName (Utilities|String|Append (Variables|Default|GetName) "K")))
    (Rendering|Components|TextRender|SetText (Variables|Default|GetNameT) (Utilities|Text|ToText(String) _output_get))))

(event Input|KeyboardEvents|L
  (params (Key :type Key%20Structure :default "AnyKey"))
  ;[1 1 1] Keyboard Events
  (:Pressed
    (bind _output_get (Variables|Default|SetName (Utilities|String|Append (Variables|Default|GetName) "L")))
    (Rendering|Components|TextRender|SetText (Variables|Default|GetNameT) (Utilities|Text|ToText(String) _output_get))))

(event Input|KeyboardEvents|M
  (params (Key :type Key%20Structure :default "AnyKey"))
  ;[1 1 1] Keyboard Events
  (:Pressed
    (bind _output_get (Variables|Default|SetName (Utilities|String|Append (Variables|Default|GetName) "M")))
    (Rendering|Components|TextRender|SetText (Variables|Default|GetNameT) (Utilities|Text|ToText(String) _output_get))))

(event Input|KeyboardEvents|N
  (params (Key :type Key%20Structure :default "AnyKey"))
  ;[1 1 1] Keyboard Events
  (:Pressed
    (bind _output_get (Variables|Default|SetName (Utilities|String|Append (Variables|Default|GetName) "N")))
    (Rendering|Components|TextRender|SetText (Variables|Default|GetNameT) (Utilities|Text|ToText(String) _output_get))))

(event Input|KeyboardEvents|O
  (params (Key :type Key%20Structure :default "AnyKey"))
  ;[1 1 1] Keyboard Events
  (:Pressed
    (bind _output_get (Variables|Default|SetName (Utilities|String|Append (Variables|Default|GetName) "O")))
    (Rendering|Components|TextRender|SetText (Variables|Default|GetNameT) (Utilities|Text|ToText(String) _output_get))))

(event Input|KeyboardEvents|Q
  (params (Key :type Key%20Structure :default "AnyKey"))
  ;[1 1 1] Keyboard Events
  (:Pressed
    (bind _output_get (Variables|Default|SetName (Utilities|String|Append (Variables|Default|GetName) "Q")))
    (Rendering|Components|TextRender|SetText (Variables|Default|GetNameT) (Utilities|Text|ToText(String) _output_get))))

(event Input|KeyboardEvents|R
  (params (Key :type Key%20Structure :default "AnyKey"))
  ;[1 1 1] Keyboard Events
  (:Pressed
    (bind _output_get (Variables|Default|SetName (Utilities|String|Append (Variables|Default|GetName) "R")))
    (Rendering|Components|TextRender|SetText (Variables|Default|GetNameT) (Utilities|Text|ToText(String) _output_get))))

(event Input|KeyboardEvents|S
  (params (Key :type Key%20Structure :default "AnyKey"))
  ;[1 1 1] Keyboard Events
  (:Pressed
    (bind _output_get (Variables|Default|SetName (Utilities|String|Append (Variables|Default|GetName) "S")))
    (Rendering|Components|TextRender|SetText (Variables|Default|GetNameT) (Utilities|Text|ToText(String) _output_get))))

(event Input|KeyboardEvents|T
  (params (Key :type Key%20Structure :default "AnyKey"))
  ;[1 1 1] Keyboard Events
  (:Pressed
    (bind _output_get (Variables|Default|SetName (Utilities|String|Append (Variables|Default|GetName) "T")))
    (Rendering|Components|TextRender|SetText (Variables|Default|GetNameT) (Utilities|Text|ToText(String) _output_get))))

(event Input|KeyboardEvents|U
  (params (Key :type Key%20Structure :default "AnyKey"))
  ;[1 1 1] Keyboard Events
  (:Pressed
    (bind _output_get (Variables|Default|SetName (Utilities|String|Append (Variables|Default|GetName) "U")))
    (Rendering|Components|TextRender|SetText (Variables|Default|GetNameT) (Utilities|Text|ToText(String) _output_get))))

(fn ConstructionScript)