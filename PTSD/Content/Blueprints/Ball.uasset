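; Ball is an interactable VR object that prompts the player to decide the fate of an item, such as a chair, fire alarm or photo.
; While Interacted, Tick snaps its Cube to the holding VRPawn's RightHolder.
; A DoOnce disables physics and collision, then spawns a DecisionUI at UISpawn with hard-coded choices and description selected by DecisionNum.
; EndObject destroys the actor.
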(event Custom|EndObject
  (Actor|DestroyActor))

(event EventTick
  (params (DeltaSeconds :type Float%20%28single-precision%29))
  (bind _returnvalue (Game|Player|GetPlayerPawn 0))
  (bind _returnvalue_2 (Game|Player|GetPlayerPawn 0))
  (bind _cube (Variables|Default|GetCube))
  (if (Variables|Default|GetInteracted)
    (bind _asvrpawn (Utilities|Casting|CastToVRPawn (Variables|Default|GetHolder)))
    (Transformation|SetWorldTransform _cube (Math|Transform|MakeTransform (.location (Transformation|GetWorldTransform (Variables|/Game/Blueprints/VRPawn.VRPawn_C|GetRightHolder _asvrpawn))) (.rotation (Transformation|GetWorldTransform (Variables|/Game/Blueprints/VRPawn.VRPawn_C|GetRightHolder _asvrpawn))) (Transformation|GetWorldScale _cube)) false false)
    (Utilities|FlowControl|DoOnce false
      (:Completed
        (Physics|SetSimulatePhysics _cube false)
        (Collision|SetCollisionEnabled _cube "NoCollision")
        (bind _returnvalue_3 (Game|SpawnActorfromClass "/Game/Blueprints/DecisionUI.DecisionUI_C" (Transformation|GetActorTransform (Variables|Default|GetUI%20Spawn)) "Undefined" 0 0))
        (if (== (Variables|Default|GetDecisionNum) 0)
          (Variables|/Game/Blueprints/DecisionUI.DecisionUI_C|SetDecisionName _returnvalue_3 "Chair: ")
          (Rendering|Components|TextRender|SetText (Variables|/Game/Blueprints/DecisionUI.DecisionUI_C|GetDecisionText1 _returnvalue_3) (Utilities|Text|ToText(String) "Throw away"))
          (Rendering|Components|TextRender|SetText (Variables|/Game/Blueprints/DecisionUI.DecisionUI_C|GetDecisionText2 _returnvalue_3) (Utilities|Text|ToText(String) "Keep"))
          (Rendering|Components|TextRender|SetText (Variables|/Game/Blueprints/DecisionUI.DecisionUI_C|GetDecisionText3 _returnvalue_3) (Utilities|Text|ToText(String) "Give To Charity"))
          (Rendering|Components|TextRender|SetText (Variables|/Game/Blueprints/DecisionUI.DecisionUI_C|GetDecisionText4 _returnvalue_3) (Utilities|Text|ToText(String) ""))
          (Rendering|Components|TextRender|SetText (Variables|/Game/Blueprints/DecisionUI.DecisionUI_C|GetLine1 _returnvalue_3) (Utilities|Text|ToText(String) ""))
          (Rendering|Components|TextRender|SetText (Variables|/Game/Blueprints/DecisionUI.DecisionUI_C|GetLine2 _returnvalue_3) (Utilities|Text|ToText(String) ""))
          (Rendering|Components|TextRender|SetText (Variables|/Game/Blueprints/DecisionUI.DecisionUI_C|GetLine3 _returnvalue_3) (Utilities|Text|ToText(String) ""))
          (Rendering|Components|TextRender|SetText (Variables|/Game/Blueprints/DecisionUI.DecisionUI_C|GetLine4 _returnvalue_3) (Utilities|Text|ToText(String) ""))
          (Rendering|Components|TextRender|SetText (Variables|/Game/Blueprints/DecisionUI.DecisionUI_C|GetLine5 _returnvalue_3) (Utilities|Text|ToText(String) ""))
          (Utilities|Casting|CastToVRPawn _returnvalue_2)
          (elif (== (Variables|Default|GetDecisionNum) 1)
            (Variables|/Game/Blueprints/DecisionUI.DecisionUI_C|SetDecisionName _returnvalue_3 "FireAlarm: ")
            (Rendering|Components|TextRender|SetText (Variables|/Game/Blueprints/DecisionUI.DecisionUI_C|GetDecisionText1 _returnvalue_3) (Utilities|Text|ToText(String) "Repair"))
            (Rendering|Components|TextRender|SetText (Variables|/Game/Blueprints/DecisionUI.DecisionUI_C|GetDecisionText2 _returnvalue_3) (Utilities|Text|ToText(String) "Throw Away"))
            (Rendering|Components|TextRender|SetText (Variables|/Game/Blueprints/DecisionUI.DecisionUI_C|GetDecisionText3 _returnvalue_3) (Utilities|Text|ToText(String) "Do Nothing"))
            (Rendering|Components|TextRender|SetText (Variables|/Game/Blueprints/DecisionUI.DecisionUI_C|GetDecisionText4 _returnvalue_3) (Utilities|Text|ToText(String) ""))
            (Rendering|Components|TextRender|SetText (Variables|/Game/Blueprints/DecisionUI.DecisionUI_C|GetLine1 _returnvalue_3) (Utilities|Text|ToText(String) "A torn-out fire alarm. It’s been removed from the wall, but still seems functional."))
            (Rendering|Components|TextRender|SetText (Variables|/Game/Blueprints/DecisionUI.DecisionUI_C|GetLine2 _returnvalue_3) (Utilities|Text|ToText(String) "Plugging it back in would probably trigger a loud test noise."))
            (Rendering|Components|TextRender|SetText (Variables|/Game/Blueprints/DecisionUI.DecisionUI_C|GetLine3 _returnvalue_3) (Utilities|Text|ToText(String) "Perhaps it would be better to throw it out and get a new one…"))
            (Rendering|Components|TextRender|SetText (Variables|/Game/Blueprints/DecisionUI.DecisionUI_C|GetLine4 _returnvalue_3) (Utilities|Text|ToText(String) ""))
            (Rendering|Components|TextRender|SetText (Variables|/Game/Blueprints/DecisionUI.DecisionUI_C|GetLine5 _returnvalue_3) (Utilities|Text|ToText(String) "What would you like to do with this? "))
            (Utilities|Casting|CastToVRPawn _returnvalue_2)
            (elif (== (Variables|Default|GetDecisionNum) 2)
              (Variables|/Game/Blueprints/DecisionUI.DecisionUI_C|SetDecisionName _returnvalue_3 "Picture1: ")
              (Rendering|Components|TextRender|SetText (Variables|/Game/Blueprints/DecisionUI.DecisionUI_C|GetDecisionText1 _returnvalue_3) (Utilities|Text|ToText(String) "Throw away"))
              (Rendering|Components|TextRender|SetText (Variables|/Game/Blueprints/DecisionUI.DecisionUI_C|GetDecisionText2 _returnvalue_3) (Utilities|Text|ToText(String) "Keep"))
              (Rendering|Components|TextRender|SetText (Variables|/Game/Blueprints/DecisionUI.DecisionUI_C|GetDecisionText3 _returnvalue_3) (Utilities|Text|ToText(String) "Donte"))
              (Rendering|Components|TextRender|SetText (Variables|/Game/Blueprints/DecisionUI.DecisionUI_C|GetDecisionText4 _returnvalue_3) (Utilities|Text|ToText(String) "Do Nothing"))
              (Rendering|Components|TextRender|SetText (Variables|/Game/Blueprints/DecisionUI.DecisionUI_C|GetLine1 _returnvalue_3) (Utilities|Text|ToText(String) "An image of a MiG-15 with its pilot."))
              (Rendering|Components|TextRender|SetText (Variables|/Game/Blueprints/DecisionUI.DecisionUI_C|GetLine2 _returnvalue_3) (Utilities|Text|ToText(String) "The photograph dates back to the Cold War, but it’s been well-kept and must be important to someone."))
              (Rendering|Components|TextRender|SetText (Variables|/Game/Blueprints/DecisionUI.DecisionUI_C|GetLine3 _returnvalue_3) (Utilities|Text|ToText(String) "No doubt the person in the photo is a beloved friend or family member. 
"))
              (Rendering|Components|TextRender|SetText (Variables|/Game/Blueprints/DecisionUI.DecisionUI_C|GetLine4 _returnvalue_3) (Utilities|Text|ToText(String) ""))
              (Rendering|Components|TextRender|SetText (Variables|/Game/Blueprints/DecisionUI.DecisionUI_C|GetLine5 _returnvalue_3) (Utilities|Text|ToText(String) "What would you like to do with this?"))
              (Utilities|Casting|CastToVRPawn _returnvalue)
              (elif (== (Variables|Default|GetDecisionNum) 3)
                (Variables|/Game/Blueprints/DecisionUI.DecisionUI_C|SetDecisionName _returnvalue_3 "Picture2:  ")
                (Rendering|Components|TextRender|SetText (Variables|/Game/Blueprints/DecisionUI.DecisionUI_C|GetDecisionText1 _returnvalue_3) (Utilities|Text|ToText(String) "Throw away"))
                (Rendering|Components|TextRender|SetText (Variables|/Game/Blueprints/DecisionUI.DecisionUI_C|GetDecisionText2 _returnvalue_3) (Utilities|Text|ToText(String) "Keep"))
                (Rendering|Components|TextRender|SetText (Variables|/Game/Blueprints/DecisionUI.DecisionUI_C|GetDecisionText3 _returnvalue_3) (Utilities|Text|ToText(String) "Do Nothing"))
                (Rendering|Components|TextRender|SetText (Variables|/Game/Blueprints/DecisionUI.DecisionUI_C|GetDecisionText4 _returnvalue_3) (Utilities|Text|ToText(String) ""))
                (Rendering|Components|TextRender|SetText (Variables|/Game/Blueprints/DecisionUI.DecisionUI_C|GetLine1 _returnvalue_3) (Utilities|Text|ToText(String) "A generic nature photo."))
                (Rendering|Components|TextRender|SetText (Variables|/Game/Blueprints/DecisionUI.DecisionUI_C|GetLine2 _returnvalue_3) (Utilities|Text|ToText(String) " There is no subject or focus, but it looks nice enough to be framed. "))
                (Rendering|Components|TextRender|SetText (Variables|/Game/Blueprints/DecisionUI.DecisionUI_C|GetLine3 _returnvalue_3) (Utilities|Text|ToText(String) "Perhaps someone took this during a trip to the outdoors. "))
                (Rendering|Components|TextRender|SetText (Variables|/Game/Blueprints/DecisionUI.DecisionUI_C|GetLine4 _returnvalue_3) (Utilities|Text|ToText(String) ""))
                (Rendering|Components|TextRender|SetText (Variables|/Game/Blueprints/DecisionUI.DecisionUI_C|GetLine5 _returnvalue_3) (Utilities|Text|ToText(String) "What would you like to do with this?"))
                (Utilities|Casting|CastToVRPawn _returnvalue)))))))))

(fn ConstructionScript)