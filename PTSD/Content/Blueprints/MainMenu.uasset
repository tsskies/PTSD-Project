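; In-world VR menu actor with three buttons that quit the game, start the game through VRPawn, or close the menu.
; Overlapping a button's collision component swaps its mesh to a hover material and records it in CurrentlyOver; leaving restores the material and clears the selection.
; Interact acts on CurrentlyOver, with Return destroying the actor.
; The Exit and Return mesh names are crossed relative to their overlap components.
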(event OnComponentBeginOverlap(ExitBox)
  (params (OverlappedComponent :type Primitive%20Component%20Object%20Reference) (OtherActor :type Actor%20Object%20Reference) (OtherComp :type Primitive%20Component%20Object%20Reference) (OtherBodyIndex :type Integer) (bFromSweep :type Boolean) (SweepResult :type Hit%20Result%20Structure%20%28by%20ref%29))
  (Rendering|Material|SetMaterial (Variables|Default|GetReturn) 0 "/Game/Textures/UI/button_hover_Mat.button_hover_Mat")
  (Variables|Default|SetCurrently%20Over "Exit"))

(event OnComponentBeginOverlap(MainB)
  (params (OverlappedComponent :type Primitive%20Component%20Object%20Reference) (OtherActor :type Actor%20Object%20Reference) (OtherComp :type Primitive%20Component%20Object%20Reference) (OtherBodyIndex :type Integer) (bFromSweep :type Boolean) (SweepResult :type Hit%20Result%20Structure%20%28by%20ref%29))
  (Rendering|Material|SetMaterial (Variables|Default|GetMainMenu) 0 "/Game/Textures/UI/button_hover_Mat.button_hover_Mat")
  (Variables|Default|SetCurrently%20Over "Main"))

(event OnComponentBeginOverlap(Returnb)
  (params (OverlappedComponent :type Primitive%20Component%20Object%20Reference) (OtherActor :type Actor%20Object%20Reference) (OtherComp :type Primitive%20Component%20Object%20Reference) (OtherBodyIndex :type Integer) (bFromSweep :type Boolean) (SweepResult :type Hit%20Result%20Structure%20%28by%20ref%29))
  (Rendering|Material|SetMaterial (Variables|Default|GetExit) 0 "/Game/Textures/UI/button_hover_Mat.button_hover_Mat")
  (Variables|Default|SetCurrently%20Over "Return"))

(event OnComponentEndOverlap(ExitBox)
  (params (OverlappedComponent :type Primitive%20Component%20Object%20Reference) (OtherActor :type Actor%20Object%20Reference) (OtherComp :type Primitive%20Component%20Object%20Reference) (OtherBodyIndex :type Integer))
  (Rendering|Material|SetMaterial (Variables|Default|GetReturn) 0 "/Game/Textures/UI/button_normal_Mat.button_normal_Mat")
  (Variables|Default|SetCurrently%20Over "none"))

(event OnComponentEndOverlap(MainB)
  (params (OverlappedComponent :type Primitive%20Component%20Object%20Reference) (OtherActor :type Actor%20Object%20Reference) (OtherComp :type Primitive%20Component%20Object%20Reference) (OtherBodyIndex :type Integer))
  (Rendering|Material|SetMaterial (Variables|Default|GetMainMenu) 0 "/Game/Textures/UI/button_normal_Mat.button_normal_Mat")
  (Variables|Default|SetCurrently%20Over "none"))

(event OnComponentEndOverlap(Returnb)
  (params (OverlappedComponent :type Primitive%20Component%20Object%20Reference) (OtherActor :type Actor%20Object%20Reference) (OtherComp :type Primitive%20Component%20Object%20Reference) (OtherBodyIndex :type Integer))
  (Rendering|Material|SetMaterial (Variables|Default|GetExit) 0 "/Game/Textures/UI/button_normal_Mat.button_normal_Mat")
  (Variables|Default|SetCurrently%20Over "none"))

(event Custom|Interact
  (switch string (Variables|Default|GetCurrently%20Over)
    (:Exit
      (Game|QuitGame 0 "Quit"))
    (:Main
      (bind _asvrpawn (Utilities|Casting|CastToVRPawn (Game|Player|GetPlayerPawn 0)))
      (Default|StartGame _asvrpawn))
    (:Return
      (Actor|DestroyActor))))

(fn ConstructionScript)